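; Player controller for the menus that opens the main menu and relays lobby player list updates to the UI.
; On BeginPlay it creates the main menu widget, adds it to the viewport, sets Game and UI input focused on it, and shows the cursor.
; UpdatePlayerList stores the received player info and passes it to the nested host lobby widget.
; A separate isClient event uses an authority switch to set the IsServer flag.
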(event Custom|isClient
  (Networking|SwitchHasAuthority
    (:Authority
      (Variables|Default|SetisServer true))
    (:Remote
      (Variables|Default|SetisServer false))))

(event Custom|UpdatePlayerList
  (params (PlayerInfo :type Array%20of%20Player%20Info%20S%20Structures))
  (bind _output_get (Variables|Default|SetConnectedPlayerInfo PlayerInfo))
  (Default|UpdatePlayerList (Variables|/Game/Blueprints/Menus/UI_Widgets/MainMenu_W.MainMenu_W_C|GetHostLobby_W (Variables|Default|GetLobbyWidget)) _output_get))

(event EventBeginPlay
  (bind _returnvalue (Game|GetPlayerController 0))
  (bind _returnvalue_2 (UserInterface|CreateWidget "/Game/Blueprints/Menus/UI_Widgets/MainMenu_W.MainMenu_W_C"))
  (bind _output_get (Variables|Default|SetLobbyWidget _returnvalue_2))
  (UserInterface|Viewport|AddtoViewport _output_get 0)
  (Input|SetInputModeGameandUI _returnvalue _output_get "DoNotLock" false false)
  (Variables|/Script/Engine.PlayerController|SetbShowMouseCursor _returnvalue true))

(fn ConstructionScript)