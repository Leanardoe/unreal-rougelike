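; MainMenu_GM is the main menu game mode that keeps the list of connected players and their Steam identities.
; On login it stores the Menu_PC and adds its Steam name and medium avatar to PlayerInfo, even if the avatar fetch fails.
; On logout it removes the controller and attempts to remove a name-only info struct.
; Both paths then push the list to every controller after a short delay.
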(event EventPostLogin
  (params (NewPlayer :type Player%20Controller%20Object%20Reference))
  (bind _asmenu_pc (Utilities|Casting|CastToMenu_PC NewPlayer))
  (Utilities|Array|Add (Variables|Default|GetConnectedPlayer) _asmenu_pc)
  (bind _returnvalue (Class|AdvancedSteamFriendsLibrary|GetSteamPersonaName (Class|AdvancedSessionsLibrary|GetUniqueNetID _asmenu_pc)))
  (bind _returnvalue_2 (Class|AdvancedSteamFriendsLibrary|GetSteamFriendAvatar (Class|AdvancedSessionsLibrary|GetUniqueNetID _asmenu_pc) "SteamAvatar_Medium")
    (:OnSuccess
      _)
    (:OnFailure
      _))
  (Utilities|Array|Add (Variables|Default|GetPlayerInfo) (Utilities|Struct|MakePlayerInfo_S (Utilities|Text|ToText(String) _returnvalue) _returnvalue_2))
  (Utilities|FlowControl|Delay 0.2)
  (for _array_element (Variables|Default|GetConnectedPlayer)
    (Default|UpdatePlayerList _array_element (Variables|Default|GetPlayerInfo))))

(event EventOnLogout
  (params (ExitingController :type Controller%20Object%20Reference))
  (bind _asmenu_pc (Utilities|Casting|CastToMenu_PC ExitingController))
  (Utilities|Array|RemoveItem (Variables|Default|GetConnectedPlayer) _asmenu_pc)
  (bind _returnvalue (Class|AdvancedSteamFriendsLibrary|GetSteamPersonaName (Class|AdvancedSessionsLibrary|GetUniqueNetID _asmenu_pc)))
  (Utilities|Array|RemoveItem (Variables|Default|GetPlayerInfo) (Utilities|Struct|MakePlayerInfo_S (Utilities|Text|ToText(String) _returnvalue)))
  (Utilities|FlowControl|Delay 0.2)
  (for _array_element (Variables|Default|GetConnectedPlayer)
    (Default|UpdatePlayerList _array_element (Variables|Default|GetPlayerInfo))))

(fn ConstructionScript)