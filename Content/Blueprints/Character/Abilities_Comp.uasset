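; Player ability component that handles level-up upgrade picks and timer-driven automatic attacks.
; BeginPlay filters the ability data table by class, and LevelUp offers three distinct rarity-weighted picks in a widget.
; SelectAbility raises skill levels, retiring them at ten, or applies stat and modifier upgrades.
; Grant functions start looping cooldown timers; Arrow fires per level at on-screen enemies with pierce and optional homing, while Slash, Bash and Fireball events are empty.
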(event Custom|Level%20Up
  (bind _returnvalue (Components|GetOwner))
  (bind _asmain_pc (Utilities|Casting|CastToMainPC _returnvalue))
  (bind (_op1 _op2 _op3) (CallFunction|RandomAbilities))
  (bind _returnvalue_2 (UserInterface|CreateWidget "/Game/Blueprints/Menus/PlayerHUD/PlayerAbilitySelect_W.PlayerAbilitySelect_W_C" 0 _asmain_pc _op1 _op2 _op3))
  (UserInterface|Viewport|AddtoViewport _returnvalue_2 0)
  (Variables|/Game/Blueprints/Character/MainPC.MainPC_C|SetiFrame _asmain_pc true)
  (Input|DisableInput _asmain_pc 0)
  (Variables|/Script/Engine.PlayerController|SetbShowMouseCursor (.AsPlayer%20Controller (Utilities|Casting|CastToPlayerController (Pawn|GetController _asmain_pc))) true))

(event EventBeginPlay
  (bind _outrownames (DataTable|GetDataTableRowNames "/Game/Blueprints/Abilities/Abilities_DT.Abilities_DT"))
  (for _array_element _outrownames
    (bind _returnvalue (Utilities|GetDataTableRow "/Game/Blueprints/Abilities/Abilities_DT.Abilities_DT" _array_element)
      (:then
        (if (or (Utilities|Enum|Equal(Enum) (Variables|/Game/Blueprints/Character/MainPC.MainPC_C|GetClass (.AsMain%20PC (Utilities|Casting|CastToMainPC (Components|GetOwner)))) (.Class (Utilities|Struct|BreakAbility_S _returnvalue))) (Utilities|Enum|Equal(Enum) (.Class (Utilities|Struct|BreakAbility_S _returnvalue)) "All"))
          (Utilities|Array|Add (Variables|Default|GetAvailableAbilities) _returnvalue))))))

(fn TargetEnemy
  (bind _returnvalue (Viewport|GetViewportSize))
  (Utilities|Array|Clear (Variables|Default|GetTargetList))
  (bind _outactors (Actor|GetAllActorsOfClass "/Game/Blueprints/Monster/EnemyBase_BP.EnemyBase_BP_C"))
  (for _array_element _outactors
    (if (and (Math|Float|InRange(Float) (.x (.ScreenLocation (Class|PlayerController|ProjectWorldLocationtoScreen (Game|GetPlayerController 0) (Transformation|GetActorLocation _array_element) false))) 0.0 (.x _returnvalue)) (Math|Float|InRange(Float) (.y (.ScreenLocation (Class|PlayerController|ProjectWorldLocationtoScreen (Game|GetPlayerController 0) (Transformation|GetActorLocation _array_element) false))) 0.0 (.y _returnvalue)))
      (Utilities|IsValid (Variables|Default|GetClosestEnemy)
        (:Is%20Valid
          (if (< (Transformation|GetDistanceTo (Game|GetPlayerController 0) (Variables|Default|GetClosestEnemy)) (Transformation|GetDistanceTo (Game|GetPlayerController 0) _array_element))
            (Utilities|Array|Add (Variables|Default|GetTargetList) _array_element)
            (else
              (bind _output_get (Variables|Default|SetClosestEnemy _array_element))
              (Utilities|Array|Insert (Variables|Default|GetTargetList) _output_get))))
        (:Is%20Not%20Valid
          (bind _output_get_2 (Variables|Default|SetClosestEnemy _array_element))
          (Utilities|Array|Insert (Variables|Default|GetTargetList) _output_get_2))))))

(fn GetTarget
  (for _array_element (Variables|Default|GetTargetList)
    _))

(fn RandomAbilities
  (bind _randabilities (LocalVariables|GetRandAbilities))
  (bind _randabilities_2 (LocalVariables|GetRandAbilities))
  (bind _levelupabilities (Variables|Default|GetLevelUpAbilities))
  (bind _randabilities_3 (LocalVariables|GetRandAbilities))
  (Utilities|Array|Clear (Variables|Default|GetLevelUpAbilities))
  (for _array_element (Variables|Default|GetAvailableAbilities)
    (for _index (range 0 (- (.Rarity (Utilities|Struct|BreakAbility_S _array_element)) 1))
      (Utilities|Array|Add (LocalVariables|GetRandAbilities) _array_element)))
  (LocalVariables|SetAbility (.OutItem (Utilities|Array|Random _randabilities)))
  (for _array_element_2 _randabilities
    (if (Utilities|Enum|Equal(Enum) (.Name (Utilities|Struct|BreakAbility_S _array_element_2)) (.Name (Utilities|Struct|BreakAbility_S (LocalVariables|GetAbility))))
      (Utilities|Array|RemoveItem (LocalVariables|GetRandAbilities) _array_element_2)))
  (Utilities|Array|Add (Variables|Default|GetLevelUpAbilities) (LocalVariables|GetAbility))
  (LocalVariables|SetAbility (.OutItem (Utilities|Array|Random _randabilities_2)))
  (for _array_element_3 _randabilities_2
    (if (Utilities|Enum|Equal(Enum) (.Name (Utilities|Struct|BreakAbility_S _array_element_3)) (.Name (Utilities|Struct|BreakAbility_S (LocalVariables|GetAbility))))
      (Utilities|Array|RemoveItem (LocalVariables|GetRandAbilities) _array_element_3)))
  (Utilities|Array|Add (Variables|Default|GetLevelUpAbilities) (LocalVariables|GetAbility))
  (LocalVariables|SetAbility (.OutItem (Utilities|Array|Random _randabilities_3)))
  (for _array_element_4 _randabilities_3
    (if (Utilities|Enum|Equal(Enum) (.Name (Utilities|Struct|BreakAbility_S _array_element_4)) (.Name (Utilities|Struct|BreakAbility_S (LocalVariables|GetAbility))))
      (Utilities|Array|RemoveItem (LocalVariables|GetRandAbilities) _array_element_4)))
  (Utilities|Array|Add (Variables|Default|GetLevelUpAbilities) (LocalVariables|GetAbility))
  (return (.Name (Utilities|Struct|BreakAbility_S (Utilities|Array|Get(acopy) _levelupabilities))) (.Name (Utilities|Struct|BreakAbility_S (Utilities|Array|Get(acopy) _levelupabilities 1))) (.Name (Utilities|Struct|BreakAbility_S (Utilities|Array|Get(acopy) _levelupabilities 2)))))

(fn GrantArrow
  (bind _aqcuiredabilities (Variables|Default|GetAqcuiredAbilities))
  (bind _returnvalue (Utilities|GetDataTableRow "/Game/Blueprints/Abilities/Abilities_DT.Abilities_DT" "Arrow")
    (:then
      (bind _returnvalue_2 (Utilities|Array|Add _aqcuiredabilities _returnvalue))
      (Math|Integer|IncrementInt (.Level (Utilities|Struct|BreakAbility_S (Utilities|Array|Get(acopy) _aqcuiredabilities _returnvalue_2)))
        (:%20%20
          (Utilities|Time|SetTimerbyFunctionName 0 "Arrow_Prep" (Variables|Default|GetSkillCD) true)
          (CallFunction|ArrowPrep))))))

(fn GrantSlash
  (bind _aqcuiredabilities (Variables|Default|GetAqcuiredAbilities))
  (bind _returnvalue (Utilities|GetDataTableRow "/Game/Blueprints/Abilities/Abilities_DT.Abilities_DT" "Slash")
    (:then
      (bind _returnvalue_2 (Utilities|Array|Add _aqcuiredabilities _returnvalue))
      (Math|Integer|IncrementInt (.Level (Utilities|Struct|BreakAbility_S (Utilities|Array|Get(acopy) _aqcuiredabilities _returnvalue_2)))
        (:%20%20
          (Utilities|Time|SetTimerbyFunctionName 0 "Slash_Prep" (Variables|Default|GetSkillCD) true)
          (CallFunction|SlashPrep))))))

(fn GrantBash
  (bind _aqcuiredabilities (Variables|Default|GetAqcuiredAbilities))
  (bind _returnvalue (Utilities|GetDataTableRow "/Game/Blueprints/Abilities/Abilities_DT.Abilities_DT" "Bash")
    (:then
      (bind _returnvalue_2 (Utilities|Array|Add _aqcuiredabilities _returnvalue))
      (Math|Integer|IncrementInt (.Level (Utilities|Struct|BreakAbility_S (Utilities|Array|Get(acopy) _aqcuiredabilities _returnvalue_2)))
        (:%20%20
          (Utilities|Time|SetTimerbyFunctionName 0 "Bash_Prep" (Variables|Default|GetSkillCD) true)
          (CallFunction|BashPrep))))))

(fn GrantFireball
  (bind _aqcuiredabilities (Variables|Default|GetAqcuiredAbilities))
  (bind _returnvalue (Utilities|GetDataTableRow "/Game/Blueprints/Abilities/Abilities_DT.Abilities_DT" "Fireball")
    (:then
      (bind _returnvalue_2 (Utilities|Array|Add _aqcuiredabilities _returnvalue))
      (Math|Integer|IncrementInt (.Level (Utilities|Struct|BreakAbility_S (Utilities|Array|Get(acopy) _aqcuiredabilities _returnvalue_2)))
        (:%20%20
          (Utilities|Time|SetTimerbyFunctionName 0 "Fireball_Prep" (Variables|Default|GetSkillCD) true)
          (CallFunction|FireballPrep))))))

(fn GetAbilityLvl
  (params (Name1 :type String))
  (for _array_element (Variables|Default|GetAqcuiredAbilities)
    (if (Utilities|Enum|Equal(Enum) Name1 (.Name (Utilities|Struct|BreakAbility_S _array_element)))
      (return (.Level (Utilities|Struct|BreakAbility_S _array_element))))))

(fn SelectAbility
  (params (Name :type String))
  (bind _returnvalue (Components|GetOwner))
  (bind _availableabilities (Variables|Default|GetAvailableAbilities))
  (bind _availableabilities_2 (Variables|Default|GetAvailableAbilities))
  (bind _asmain_pc (Utilities|Casting|CastToMainPC _returnvalue))
  (for (_array_element _array_index) (Variables|Default|GetAqcuiredAbilities)
    (if (Utilities|Enum|Equal(Enum) (.Name (Utilities|Struct|BreakAbility_S _array_element)) Name)
      (Variables|Default|SetHasAbility true)
      (LocalVariables|SetArrayItem _array_index)))
  (switch string Name
    (:Arrow
      (if (Variables|Default|GetHasAbility)
        (bind _result (Math|Integer|IncrementInt (.level (Utilities|Array|Get(acopy) (Variables|Default|GetAqcuiredAbilities) (LocalVariables|GetArrayItem))))
          (:%20%20
            (if (>= _result 10)
              (for (_array_element_2 _array_index_2) _availableabilities_2 :!label _label
                (if (Utilities|Enum|Equal(Enum) (.name _array_element_2) (.name (Utilities|Array|Get(acopy) (Variables|Default|GetAqcuiredAbilities) (LocalVariables|GetArrayItem))))
                  (Utilities|Array|RemoveIndex _availableabilities_2 _array_index_2))))))))
    (:Slash
      (if (Variables|Default|GetHasAbility)
        (bind _result_2 (Math|Integer|IncrementInt (.level (Utilities|Array|Get(acopy) (Variables|Default|GetAqcuiredAbilities) (LocalVariables|GetArrayItem))))
          (:%20%20
            (if (>= _result_2 10)
              (goto _label))))))
    (:Bash
      (if (Variables|Default|GetHasAbility)
        (bind _result_3 (Math|Integer|IncrementInt (.level (Utilities|Array|Get(acopy) (Variables|Default|GetAqcuiredAbilities) (LocalVariables|GetArrayItem))))
          (:%20%20
            (if (>= _result_3 10)
              (goto _label))))))
    (:Fireball
      (if true
        (bind _result_4 (Math|Integer|IncrementInt (.level (Utilities|Array|Get(acopy) (Variables|Default|GetAqcuiredAbilities) (LocalVariables|GetArrayItem))))
          (:%20%20
            (if (>= _result_4 10)
              (goto _label))))))
    (:Homing
      (Variables|Default|SetHoming true)
      (for (_array_element_3 _array_index_3) _availableabilities
        (if (Utilities|Enum|Equal(Enum) (.name _array_element_3) "Homing")
          (Utilities|Array|RemoveIndex _availableabilities _array_index_3))))
    (:Damage
      (Math|Float|IncrementFloat (Variables|/Game/Blueprints/Character/MainPC.MainPC_C|GetBaseAttack _asmain_pc)))
    (:Pierce
      (Math|Integer|IncrementInt (Variables|Default|GetPierce)))
    (:AOE
      (Variables|Default|SetAOE (+ (Variables|Default|GetAOE) (* (Variables|Default|GetAOE) 0.1))))
    (:AttackSpeed
      (Variables|Default|SetSkillCD (* (Variables|Default|GetSkillCD) 0.95)))
    (:AttackRange
      (Variables|Default|SetAttackRange (+ (Variables|Default|GetAttackRange) (* (Variables|Default|GetAttackRange) 0.1))))
    (:MoveSpeed
      (Variables|/Game/Blueprints/Character/MainPC.MainPC_C|SetSpeed _asmain_pc (+ (Variables|/Game/Blueprints/Character/MainPC.MainPC_C|GetSpeed _asmain_pc) (* (Variables|/Game/Blueprints/Character/MainPC.MainPC_C|GetSpeed _asmain_pc) 0.1))))
    (:Health
      (Variables|/Game/Blueprints/Character/MainPC.MainPC_C|SetMaxHealth _asmain_pc (+ (Variables|/Game/Blueprints/Character/MainPC.MainPC_C|GetMaxHealth _asmain_pc) (* (Variables|/Game/Blueprints/Character/MainPC.MainPC_C|GetMaxHealth _asmain_pc) 0.1))))))

(event Custom|Arrow_Prep
  (bind _returnvalue (Components|GetOwner))
  (bind _asmain_pc (Utilities|Casting|CastToMainPC _returnvalue))
  (bind _level (CallFunction|GetAbilityLvl (Variables|/Game/Blueprints/Character/MainPC.MainPC_C|GetAbilities_Comp _asmain_pc) "Arrow"))
  (for _index (range 0 (- _level 1))
    (CallFunction|TargetEnemy)
    (CallFunction|ArrowExecuteServer (Variables|/Game/Blueprints/Character/MainPC.MainPC_C|GetBaseAttack _asmain_pc) _asmain_pc (Utilities|Array|Get(acopy) (Variables|Default|GetTargetList) _index) (Variables|Default|GetPierce))))

(event Custom|Arrow_Execute_Server
  (params (Damage :type Float%20%28double-precision%29) (Player :type Main%20PC%20Object%20Reference) (Target :type Enemy%20Base%20BP%20Object%20Reference) (PierceLevel :type Integer))
  (Utilities|IsValid Target
    (:Is%20Valid
      (bind _returnvalue (Game|SpawnActorfromClass "/Game/Blueprints/Abilities/Arrow_BP_Child.Arrow_BP_Child_C" (Math|Transform|MakeTransform (Transformation|GetActorLocation Player) (Math|Rotator|FindLookatRotation (Transformation|GetActorLocation Player) (Transformation|GetActorLocation Target)) "1.000000,1.000000,1.000000") "Undefined" "MultiplyWithRoot" 0 Target PierceLevel Damage Player))
      (if (Variables|Default|GetHoming)
        (Variables|/Script/Engine.ProjectileMovementComponent|SetbIsHomingProjectile (Variables|/Game/Blueprints/Abilities/BaseProjectile_BP.BaseProjectile_BP_C|GetProjectileMovement _returnvalue) true)
        (CallFunction|ArrowMulti)))))

(event Custom|Arrow_Multi)

(event Custom|Slash_S)

(event Custom|Slash_Prep)

(event Custom|Slash_Multi)

(event Custom|Bash_Prep)

(event Custom|Bash_S)

(event Custom|Bash_Multi)

(event Custom|Fireball_Multi)

(event Custom|Fireball_Prep)

(event Custom|Fireball_S)