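; Player character for a roguelike, with Enhanced Input movement, a class-based starting ability, health and experience leveling.
; On start it creates the HUD and a Steam-named health bar, then grants the Game Instance class's ability through AbilitiesComp.
; A pickup sphere triggers gem pickup, and capsule overlap awards experience, driving level-ups and HUD updates.
; Selected upgrades adjust cooldown, pierce or max health; damage updates the bar and triggers one-time death.
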(event OnComponentBeginOverlap(PickupSphere)
  (params (OverlappedComponent :type Primitive%20Component%20Object%20Reference) (OtherActor :type Actor%20Object%20Reference) (OtherComp :type Primitive%20Component%20Object%20Reference) (OtherBodyIndex :type Integer) (bFromSweep :type Boolean) (SweepResult :type Hit%20Result%20Structure%20%28by%20ref%29))
  (bind _asexp_gem_bp (Utilities|Casting|CastToEXP_Gem_BP OtherActor)
    (:then
      (bind _output_get (Variables|Default|SetAs%20EXP%20Gem%20BP _asexp_gem_bp))
      (Default|Pickup _output_get self))
    (:CastFailed
      (bind _asgold_coin_bp (Utilities|Casting|CastToGold_Coin_BP OtherActor))
      (Variables|Default|SetAs%20Gold%20Coin%20BP _asgold_coin_bp))))

(event OnComponentBeginOverlap(CapsuleComponent)
  (params (OverlappedComponent :type Primitive%20Component%20Object%20Reference) (OtherActor :type Actor%20Object%20Reference) (OtherComp :type Primitive%20Component%20Object%20Reference) (OtherBodyIndex :type Integer) (bFromSweep :type Boolean) (SweepResult :type Hit%20Result%20Structure%20%28by%20ref%29))
  (bind _asexp_gem_bp (Utilities|Casting|CastToEXP_Gem_BP OtherActor))
  (CallFunction|EarnExperience (Variables|/Game/Blueprints/Drops/EXP_Gem_BP.EXP_Gem_BP_C|GetEXP_Value _asexp_gem_bp))
  (Actor|DestroyActor _asexp_gem_bp))

(event EventBeginPlay
  (bind _abilities_comp (Variables|Default|GetAbilities_Comp))
  (bind _asplayer_controller (Utilities|Casting|CastToPlayerController (Pawn|GetController)))
  (Input|AddMappingContext (PlayerController|LocalPlayerSubsystems|GetEnhancedInputLocalPlayerSubsystem _asplayer_controller) "/Game/Blueprints/Character/Input/Roguelike_IMC.Roguelike_IMC" 0 "(bIgnoreAllPressedKeysUntilRelease=True,bForceImmediately=False,bNotifyUserSettings=False)")
  (Utilities|FlowControl|Delay 0.5)
  (CallFunction|SetupWidgetsOC)
  (bind _returnvalue (UserInterface|CreateWidget "/Game/Blueprints/Menus/PlayerHUD/MainPlayerHUD_W.MainPlayerHUD_W_C"))
  (bind _output_get (Variables|Default|SetHUDWidgetRef _returnvalue))
  (UserInterface|Viewport|AddtoViewport _output_get 0)
  (CallFunction|UpdateHUD)
  (bind _output_get_2 (Variables|Character|SetClass (Variables|/Game/Blueprints/Rogulike_GI.Rogulike_GI_C|GetClass (.AsRogulike%20GI (Utilities|Casting|CastToRogulike_GI (Game|GetGameInstance))))))
  (switch string _output_get_2
    (:Archer
      (Default|GrantArrow _abilities_comp))
    (:Swordmaster
      (Default|GrantSlash _abilities_comp))
    (:Sheildmaster
      (Default|GrantBash _abilities_comp))
    (:Mage
      (Default|GrantFireball _abilities_comp))))

(fn ConstructionScript)

(fn CreateHealthWidget
  (bind _returnvalue (Class|AdvancedSteamFriendsLibrary|GetSteamPersonaName (Class|AdvancedSessionsLibrary|GetUniqueNetID (Game|GetPlayerController 0))))
  (bind _returnvalue_2 (UserInterface|CreateWidget "/Game/Blueprints/Menus/PlayerHUD/PlayerInfo_W.PlayerInfo_W_C" 0 (Utilities|Struct|MakePlayerInfo_S (Utilities|Text|ToText(String) _returnvalue))))
  (bind _output_get (Variables|Default|SetHealthBarWidgetRef _returnvalue_2))
  (UserInterface|SetWidget (Variables|Default|GetPlayerInfo) _output_get)
  (CallFunction|UpdateHealthMulticast (/ (Variables|Character|GetCurrentHealth) (Variables|Character|GetMaxHealth))))

(fn UpdateHUD
  (bind _hudwidgetref (Variables|Default|GetHUDWidgetRef))
  (Rendering|Components|TextRender|SetText (Variables|/Game/Blueprints/Menus/PlayerHUD/MainPlayerHUD_W.MainPlayerHUD_W_C|GetLevelText _hudwidgetref) (Utilities|Text|ToText(Integer) (Variables|Character|GetLevel)))
  (bind _expremaining (CallFunction|GetNextLevelExp))
  (Rendering|Components|TextRender|SetText (Variables|/Game/Blueprints/Menus/PlayerHUD/MainPlayerHUD_W.MainPlayerHUD_W_C|GetExpNextText _hudwidgetref) (Utilities|Text|ToText(Integer) _expremaining))
  (Rendering|Components|TextRender|SetText (Variables|/Game/Blueprints/Menus/PlayerHUD/MainPlayerHUD_W.MainPlayerHUD_W_C|GetCurrentExpText _hudwidgetref) (Utilities|Text|ToText(Integer) (Variables|Character|GetCurrentExp))))

(fn GetNextLevelExp
  (return (Math|Float|Truncate (* (+ (* (Variables|Character|GetLevel) 0.7) 1.0) 1e+01))))

(fn SelectedAbility
  (params (Selected :type Integer))
  (bind _abilities_comp (Variables|Default|GetAbilities_Comp))
  (switch int Selected
    (:1
      (Variables|/Game/Blueprints/Character/Abilities_Comp.Abilities_Comp_C|SetSkillCD _abilities_comp (- (Variables|/Game/Blueprints/Character/Abilities_Comp.Abilities_Comp_C|GetSkillCD _abilities_comp) 0.1)))
    (:2
      (Variables|/Game/Blueprints/Character/Abilities_Comp.Abilities_Comp_C|SetPierce _abilities_comp (+ (Variables|/Game/Blueprints/Character/Abilities_Comp.Abilities_Comp_C|GetPierce _abilities_comp) 1)))
    (:3
      (bind _output_get (Variables|Character|SetMaxHealth (+ (Variables|Character|GetMaxHealth) 1e+01)))
      (Variables|Character|SetCurrentHealth _output_get)
      (CallFunction|UpdateHealthMulticast 1e+02))))

(event Input|EnhancedActionEvents|EnhancedInputActionMove_IA
  (params (ActionValue :type Vector%202D%20Structure) (ElapsedSeconds :type Float%20%28double-precision%29) (TriggeredSeconds :type Float%20%28double-precision%29) (InputAction :type Input%20Action%20Object%20Reference :default "/Game/Blueprints/Character/Input/Move_IA.Move_IA"))
  (bind (_x _y) (Math|Vector2D|BreakVector2D ActionValue))
  (Pawn|Input|AddMovementInput (Math|Vector|MakeVector _x _y 0.0) (Variables|Character|GetSpeed) false))

(event Custom|Death
  (Input|DisableInput (Game|GetPlayerController 0)))

(event Custom|DeathMulti
  (Collision|SetCollisionResponsetoChannel (Variables|Collision|GetCapsuleComponent) "ECC_Pawn" "ECR_Ignore"))

(event Game|Damage|EventAnyDamage
  (params (Damage :type Float%20%28single-precision%29) (DamageType :type Damage%20Type%20Object%20Reference) (InstigatedBy :type Controller%20Object%20Reference) (DamageCauser :type Actor%20Object%20Reference))
  (bind _output_get (Variables|Character|SetCurrentHealth (- (Variables|Character|GetCurrentHealth) Damage)))
  (CallFunction|UpdateHealthMulticast (/ (Variables|Character|GetCurrentHealth) (Variables|Character|GetMaxHealth)))
  (if (<= _output_get 0.0)
    (Utilities|FlowControl|DoOnce false
      (:Completed
        (Variables|Default|SetisDead true)
        (CallFunction|Death)
        (CallFunction|DeathMulti)))))

(event Custom|UpdateHealthMulticast
  (params (Percent :type Float%20%28double-precision%29))
  (bind _healthbarwidgetref (Variables|Default|GetHealthBarWidgetRef)
    (:then
      (Progress|SetPercent (Variables|/Game/Blueprints/Menus/PlayerHUD/PlayerInfo_W.PlayerInfo_W_C|GetHPProgressBar _healthbarwidgetref) Percent))
    (:else)))

(event Custom|SetupWidgets_OC
  (CallFunction|CreateHealthWidget))

(event Custom|Earn%20Experience
  (params (Exp :type Integer))
  (Utilities|FlowControl|DoOnce false :!label _label
    (:Completed
      (bind _output_get (Variables|Character|SetCurrentExp (+ (Variables|Character|GetCurrentExp) Exp)))
      (if (>= _output_get (Variables|Character|GetExpRemaining))
        (Variables|Character|SetCurrentExp (- (Variables|Character|GetCurrentExp) (Variables|Character|GetExpRemaining)))
        (Math|Integer|IncrementInt (Variables|Character|GetLevel)
          (:%20%20
            (bind _expremaining (CallFunction|GetNextLevelExp))
            (Variables|Character|SetExpRemaining _expremaining)
            (CallFunction|UpdateHUD)
            (Default|LevelUp (Variables|Default|GetAbilities_Comp))
            (goto _label Reset)))
        (else
          (CallFunction|UpdateHUD)
          (goto _label Reset))))))