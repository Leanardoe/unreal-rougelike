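; Survivors game mode that runs enemy waves on the authority, spawning through SpawnPoint actors found at BeginPlay.
; Each wave sums EnemyPool counts and sends up to EnemyMaxCount enemies to random spawners.
; OnEnemyDefeated refills from the remainder; when none remain, it grows the cap by half and starts the next wave after a delay.
; GetEnemyFromPool always returns Bat_BP, and EndWave is empty.
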(event EventBeginPlay
  (Networking|SwitchHasAuthority
    (:Authority
      (CallFunction|GetSpawners)
      (CallFunction|NewWave))))

(fn ConstructionScript)

(fn GetSpawners
  (bind _outactors (Actor|GetAllActorsOfClass "/Game/Blueprints/SpawnPoint.SpawnPoint_C"))
  (Variables|Default|SetSpawners _outactors))

(fn StartWave
  (CallFunction|BuildEnemyPool)
  (for _index (range 0 (- (Math|Integer|Min(Integer) (CallFunction|GetPoolSize) (Variables|Default|GetEnemyMaxCount)) 1))
    (Default|AddEnemy (.OutItem (Utilities|Array|Random (Variables|Default|GetSpawners))) (CallFunction|GetEnemyfromPool))))

(fn EndWave)

(fn BuildEnemyPool
  (Variables|Default|SetEnemyRemaining (CallFunction|GetPoolSize)))

(fn GetPoolSize
  (bind _values (Utilities|Map|Values (Variables|Default|GetEnemyPool)))
  (for _array_element _values
    (LocalVariables|SetlocalSum (+ (LocalVariables|GetlocalSum) _array_element)))
  (return (LocalVariables|GetlocalSum)))

(fn GetEnemyfromPool
  (return "/Game/Blueprints/Monster/Bat/Bat_BP.Bat_BP_C"))

(fn NewWave
  (Math|Integer|IncrementInt (Variables|Default|GetWaveNum)
    (:%20%20
      (CallFunction|StartWave))))

(fn OnEnemyDefeated
  (bind _result (Math|Integer|DecrementInt (Variables|Default|GetEnemyRemaining))
    (:%20%20
      (if (< _result (Variables|Default|GetEnemyMaxCount))
        (if (<= (Variables|Default|GetEnemyRemaining) 0)
          (Variables|Default|SetEnemyMaxCount (+ (Variables|Default|GetEnemyMaxCount) (/ (Variables|Default|GetEnemyMaxCount) 2)))
          (Utilities|Time|SetTimerbyFunctionName 0 "NewWave" 5.0))
        (else
          (Default|AddEnemy (.OutItem (Utilities|Array|Random (Variables|Default|GetSpawners))) (CallFunction|GetEnemyfromPool)))))))