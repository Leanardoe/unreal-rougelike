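; Enemy spawn point actor that holds a queue of enemy classes and spawns them at its own transform, oldest first.
; A looping timer tries to spawn the next queued enemy, and AddEnemy also spawns at once when no EnemyBase_BP overlaps its sphere.
; Each spawned actor's OnDestroyed event is bound, and a defeat handler forwards to the Survivors_GM game mode.
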(event Custom|OnEnemyDefeated
  (params (DestroyedActor :type Actor%20Object%20Reference))
  (bind _assurvivors_gm (Utilities|Casting|CastToSurvivors_GM (Game|GetGameMode)))
  (Default|OnEnemyDefeated _assurvivors_gm))

(event Custom|TrytoSpawn
  (CallFunction|SpawnEnemy))

(event EventBeginPlay
  (Utilities|Time|SetTimerbyEvent (delegate Custom|TrytoSpawn) 2.0 true))

(event Collision|EventActorBeginOverlap
  (params (OtherActor :type Actor%20Object%20Reference)))

(event EventTick
  (params (DeltaSeconds :type Float%20%28single-precision%29)))

(fn ConstructionScript)

(fn SpawnEnemy
  (if (Utilities|Array|IsValidIndex (Variables|Default|GetEnemyQueue))
    (bind _returnvalue (Game|SpawnActorfromClass (Utilities|Array|Get(acopy) (Variables|Default|GetEnemyQueue)) (Transformation|GetActorTransform) "Undefined" "MultiplyWithRoot" 0 0))
    (Game|BindEventtoOnDestroyed _returnvalue (EventDispatchers|CreateEvent :!event Custom|OnEnemyDefeated))
    (Utilities|Array|RemoveIndex (Variables|Default|GetEnemyQueue))
    (return true)
    (else
      (return false))))

(fn AddEnemy
  (params (NewItem :type Enemy%20Base%20BP%20Class%20Reference%20%28by%20ref%29))
  (Utilities|Array|Add (Variables|Default|GetEnemyQueue) NewItem)
  (if (not (Utilities|Array|IsValidIndex (Collision|GetOverlappingActors (Variables|Default|GetSphere) "/Game/Blueprints/Monster/EnemyBase_BP.EnemyBase_BP_C" :!class /Script/Engine.PrimitiveComponent)))
    (CallFunction|SpawnEnemy)))