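; Base ability projectile that homes in on a target enemy's sprite, destroying itself at BeginPlay if no valid target exists.
; Overlapping the target applies damage, then either destroys the projectile or, while PierceLevel remains, decrements it and retargets.
; GetNewTarget scans all EnemyBase_BP actors for any closer in XY than the current Target, which starts as the just-hit enemy and is not excluded.
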(event EventBeginPlay
  (Utilities|IsValid (Variables|Default|GetTarget)
    (:Is%20Valid
      (Variables|/Script/Engine.ProjectileMovementComponent|SetHomingTargetComponent (Variables|Default|GetProjectileMovement) (Variables|/Script/Paper2D.PaperCharacter|GetSprite (.AsEnemy%20Base%20BP (Utilities|Casting|CastToEnemyBase_BP (Variables|Default|GetTarget))))))
    (:Is%20Not%20Valid
      (Actor|DestroyActor))))

(event Collision|EventActorBeginOverlap
  (params (OtherActor :type Actor%20Object%20Reference))
  (if (== OtherActor (Variables|Default|GetTarget))
    (if (<= (Variables|Default|GetPierceLevel) 0)
      (Game|Damage|ApplyDamage (Variables|Default|GetTarget) (Variables|Default|GetDamage) 0 0)
      (Actor|DestroyActor)
      (else
        (Game|Damage|ApplyDamage (Variables|Default|GetTarget) (Variables|Default|GetDamage) 0 0)
        (CallFunction|GetNewTarget)
        (Math|Integer|DecrementInt (Variables|Default|GetPierceLevel)
          (:%20%20
            (Variables|/Script/Engine.ProjectileMovementComponent|SetHomingTargetComponent (Variables|Default|GetProjectileMovement) (Variables|/Script/Paper2D.PaperCharacter|GetSprite (.AsEnemy%20Base%20BP (Utilities|Casting|CastToEnemyBase_BP (Variables|Default|GetTarget)))))))))))

(fn ConstructionScript)

(fn GetNewTarget
  (bind _outactors (Actor|GetAllActorsOfClass "/Game/Blueprints/Monster/EnemyBase_BP.EnemyBase_BP_C"))
  (for _array_element _outactors
    (if (CallFunction|GetDistance _array_element)
      (Variables|Default|SetTarget _array_element))))

(fn GetDistance
  (params (PotTarget :type Actor%20Object%20Reference))
  (bind _returnvalue (Transformation|GetActorLocation))
  (bind _returnvalue_2 (Transformation|GetActorLocation PotTarget))
  (bind _returnvalue_3 (Transformation|GetActorLocation))
  (bind _target (Variables|Default|GetTarget))
  (bind _returnvalue_4 (Transformation|GetActorLocation _target))
  (return (< (Math|Vector|Distance2D(Vector) (Math|Vector2D|MakeVector2D (.x _returnvalue) (.y _returnvalue)) (Math|Vector2D|MakeVector2D (.x _returnvalue_2) (.y _returnvalue_2))) (Math|Vector|Distance2D(Vector) (Math|Vector2D|MakeVector2D (.x _returnvalue_3) (.y _returnvalue_3)) (Math|Vector2D|MakeVector2D (.x _returnvalue_4) (.y _returnvalue_4))))))