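; Base enemy that chases the player seen via PawnSensing, deals contact damage and drops an EXP gem on death.
; Sight or overlap sets the MainPC target, and sightings drive AI MoveTo.
; Overlap calls DamagePlayer directly and by timer, with DoOnce and an AttackSpeed delay gating hits and player IFrames blocking damage.
; AnyDamage reduces health and handles death, while EnemyAttackMulti is an empty attack event.
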(event OnSeePawn(PawnSensing)
  (params (Pawn :type Pawn%20Object%20Reference))
  (Utilities|IsValid (Variables|Default|GetTarget)
    (:Is%20Valid
      _)
    (:Is%20Not%20Valid
      (bind _asmain_pc (Utilities|Casting|CastToMainPC Pawn))
      (Variables|Default|SetTarget _asmain_pc)))
  (CallFunction|ChasePlayer))

(event Custom|ChasePlayer
  (Utilities|IsValid (Variables|Default|GetTarget)
    (:Is%20Valid
      (AI|AIMoveTo self "0, 0, 0" (Variables|Default|GetTarget) 5.0 false))))

(event EventBeginPlay
  (Variables|/Script/Engine.CharacterMovementComponent|SetMaxWalkSpeed (Variables|Character|GetCharacterMovement) (Variables|Default|GetSpeed)))

(fn ConstructionScript)

(fn DroponDeath
  (Game|SpawnActorfromClass "/Game/Blueprints/Drops/EXP_Gem_BP.EXP_Gem_BP_C" (Math|Conversions|ToTransform(Vector) (Transformation|GetActorLocation)) "Undefined" "MultiplyWithRoot" 0 (Variables|Default|GetEXP_Value) 0))

(event Custom|DamagePlayer
  (Utilities|FlowControl|DoOnce false :!label _label
    (:Completed
      (if (not (Variables|Default|GetisDead))
        (if (Variables|/Game/Blueprints/Character/MainPC.MainPC_C|GetiFrame (Variables|Default|GetTarget))
          (Utilities|FlowControl|RetriggerableDelay (Variables|Default|GetAttackSpeed) :!label _label_2)
          (goto _label Reset)
          (else
            (Game|Damage|ApplyDamage (Variables|Default|GetTarget) (Variables|Default|GetDamage) 0 self)
            (CallFunction|EnemyAttackMulti)
            (if (Variables|/Game/Blueprints/Character/MainPC.MainPC_C|GetisDead (Variables|Default|GetTarget))
              (Utilities|Time|ClearandInvalidateTimerbyHandle (Variables|Default|GetDmgPlayerTimerRef))
              (Variables|Default|SetTarget 0)
              (else
                (goto _label_2)))))))))

(event Custom|EnemyAttackMulti)

(event Collision|EventActorBeginOverlap
  (params (OtherActor :type Actor%20Object%20Reference))
  (bind _asmain_pc (Utilities|Casting|CastToMainPC OtherActor))
  (Variables|Default|SetTarget _asmain_pc)
  (bind _returnvalue (Utilities|Time|SetTimerbyFunctionName 0 "DamagePlayer" 1.0))
  (Variables|Default|SetDmgPlayerTimerRef _returnvalue)
  (CallFunction|DamagePlayer))

(event Collision|EventActorEndOverlap
  (params (OtherActor :type Actor%20Object%20Reference))
  (if (== OtherActor (Variables|Default|GetTarget))
    (Utilities|Time|ClearandInvalidateTimerbyHandle (Variables|Default|GetDmgPlayerTimerRef))))

(event Game|Damage|EventAnyDamage
  (params (Damage :type Float%20%28single-precision%29) (DamageType :type Damage%20Type%20Object%20Reference) (InstigatedBy :type Controller%20Object%20Reference) (DamageCauser :type Actor%20Object%20Reference))
  (Variables|Default|SetCurrentHealth (- (Variables|Default|GetCurrentHealth) Damage))
  (if (<= (- (Variables|Default|GetCurrentHealth) Damage) 0.0)
    (CallFunction|DroponDeath)
    (Actor|DestroyActor)))